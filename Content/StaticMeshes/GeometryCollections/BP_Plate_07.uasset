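; Breakable plate prop that the player's Cat can knock with a hit press to cause chaos.
; On BeginPlay it binds to the Cat's hit-press event, while a Box trigger tracks an overlap flag without filtering the overlapping actor.
; A press during overlap applies a fixed horizontal impulse to the Geometry Collection at the actor's location and raises the Cat's ChaosCaused.
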(event OnComponentBeginOverlap(Box)
  (params (OverlappedComponent :type Primitive%20Component%20Object%20Reference) (OtherActor :type Actor%20Object%20Reference) (OtherComp :type Primitive%20Component%20Object%20Reference) (OtherBodyIndex :type Integer) (bFromSweep :type Boolean) (SweepResult :type Hit%20Result%20Structure%20%28by%20ref%29))
  (Variables|Default|SetIsOverlap true))

(event OnComponentEndOverlap(Box)
  (params (OverlappedComponent :type Primitive%20Component%20Object%20Reference) (OtherActor :type Actor%20Object%20Reference) (OtherComp :type Primitive%20Component%20Object%20Reference) (OtherBodyIndex :type Integer))
  (Variables|Default|SetIsOverlap false))

(event Custom|ObjectPushed
  (if (Variables|Default|GetIsOverlap)
    (Physics|AddImpulseatLocation (Variables|Default|GetGeometryCollection) "400000.000000,400000.000000,0.000000" (Transformation|GetActorLocation) "None")
    (bind _ascat (Utilities|Casting|CastToCat (Game|GetPlayerCharacter 0)))
    (Variables|/Game/ThirdPerson/Blueprints/Cat.Cat_C|SetChaosCaused _ascat (+ (Variables|/Game/ThirdPerson/Blueprints/Cat.Cat_C|GetChaosCaused _ascat) 0.1))))

(event EventBeginPlay
  (bind _ascat (Utilities|Casting|CastToCat (Game|GetPlayerCharacter 0)))
  (EventDispatchers|BindEventtoHitPress _ascat (delegate Custom|ObjectPushed)))

(event Collision|EventActorBeginOverlap
  (params (OtherActor :type Actor%20Object%20Reference)))

(fn ConstructionScript)