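; BP_Plate_05 is a breakable plate Geometry Collection that the Cat player can knock apart to cause chaos.
; A box overlap sets a flag and shows the W_Break_Object widget, removing it on exit.
; On BeginPlay it applies a small impulse and binds to the Cat's HitPress event.
; A press during overlap applies a much larger impulse, raises the Cat's ChaosCaused and destroys the actor after a delay.
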(event OnComponentBeginOverlap(Box)
  (params (OverlappedComponent :type Primitive%20Component%20Object%20Reference) (OtherActor :type Actor%20Object%20Reference) (OtherComp :type Primitive%20Component%20Object%20Reference) (OtherBodyIndex :type Integer) (bFromSweep :type Boolean) (SweepResult :type Hit%20Result%20Structure%20%28by%20ref%29))
  (Variables|Default|SetIsOverlap true)
  (bind _returnvalue (UserInterface|CreateWidget "/Game/HUD/W_Break_Object.W_Break_Object_C"))
  (UserInterface|Viewport|AddtoViewport _returnvalue 0))

(event OnComponentEndOverlap(Box)
  (params (OverlappedComponent :type Primitive%20Component%20Object%20Reference) (OtherActor :type Actor%20Object%20Reference) (OtherComp :type Primitive%20Component%20Object%20Reference) (OtherBodyIndex :type Integer))
  (Variables|Default|SetIsOverlap false)
  (bind _foundwidgets (Widget|GetAllWidgetsOfClass "/Game/HUD/W_Break_Object.W_Break_Object_C" true))
  (Widget|RemovefromParent (Utilities|Array|Get(acopy) _foundwidgets)))

(event Custom|ObjectPushed
  (if (Variables|Default|GetIsOverlap)
    (Physics|AddImpulseatLocation (Variables|Default|GetGeometryCollection) "500000.000000,-500000.000000,0.000000" (Transformation|GetActorLocation) "None")
    (bind _ascat (Utilities|Casting|CastToCat (Game|GetPlayerCharacter 0)))
    (Variables|/Game/ThirdPerson/Blueprints/Cat.Cat_C|SetChaosCaused _ascat (+ (Variables|/Game/ThirdPerson/Blueprints/Cat.Cat_C|GetChaosCaused _ascat) 0.1))
    (Utilities|FlowControl|Delay 2.0)
    (Actor|DestroyActor)))

(event EventBeginPlay
  (Physics|AddImpulseatLocation (Variables|Default|GetGeometryCollection) "30000.000000,-30000.000000,0.000000" (Transformation|GetActorLocation) "None")
  (bind _ascat (Utilities|Casting|CastToCat (Game|GetPlayerCharacter 0)))
  (EventDispatchers|BindEventtoHitPress _ascat (delegate Custom|ObjectPushed)))

(event Collision|EventActorBeginOverlap
  (params (OtherActor :type Actor%20Object%20Reference)))

(fn ConstructionScript)